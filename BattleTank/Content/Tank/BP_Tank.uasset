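; BP_Tank is a player-controllable tank pawn that drives, aims and fires.
; BeginPlay hands the turret and barrel to the TankAiming component and both tracks to TankMovement.
; Move, turn and fire inputs go to those components, while aim axes rotate an azimuth gimbal and spring arm, scaled by frame time.
; Per-track throttle inputs are stubs, with their SetThrottle calls left disconnected.
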(event `self.ReceiveBeginPlay`
  (`TankAimingComponent.Initialize` (`self.TankAiming`) (`self.TankTurret`) (`self.TankBarrel`))
  (`TankMovementComponent.Initialize` (`self.TankMovement`) (`self.LeftTrack`) (`self.RightTrack`)))

(event `InputAxis|LeftTrackThrottle`
  (params (AxisValue :type "Float (single-precision)"))
  ;[1 1 1] Movement
)

(event `InputAxis|AimAzimuth`
  (params (AxisValue :type "Float (single-precision)"))
  ;[1 1 1] Aim
  (`SceneComponent.K2_AddLocalRotation` (`self.AzimuthGimble`) (`KismetMathLibrary.MakeRotator` 0.0 0.0 (* AxisValue (`GameplayStatics.GetWorldDeltaSeconds`) 100.0)) false false))

(event `InputAxis|RightTrackThrottle`
  (params (AxisValue :type "Float (single-precision)"))
  ;[1 1 1] Movement
)

(event `InputAxis|AimAltitude`
  (params (AxisValue :type "Float (single-precision)"))
  ;[1 1 1] Aim
  (`SceneComponent.K2_AddLocalRotation` (`self.SpringArm`) (`KismetMathLibrary.MakeRotator` 0.0 (* AxisValue (`GameplayStatics.GetWorldDeltaSeconds`) 100.0)) false false))

(event `InputAxis|MoveForward`
  (params (AxisValue :type "Float (single-precision)"))
  ;[1 1 1] Movement
  (`TankMovementComponent.IntendMoveForward` (`self.TankMovement`) AxisValue))

(event `InputAxis|TurnRight`
  (params (AxisValue :type "Float (single-precision)"))
  ;[1 1 1] Movement
  (`TankMovementComponent.IntendTurnRight` (`self.TankMovement`) AxisValue))

(event `InputAction|Fire`
  (params (Key :type "Key Structure"))
  ;[1 1 1] Aim
  (:`Pressed`
    (`TankAimingComponent.Fire` (`self.TankAiming`))))

(fn `UserConstructionScript`)